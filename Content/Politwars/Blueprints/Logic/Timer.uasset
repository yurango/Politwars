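; Timer Blueprint that shows an in-world countdown on the TextTimer text component.
; StartTimer waits briefly, reveals the text, then plays the CountdownTimer timeline in reverse from its end.
; Each update turns the timeline value into a minutes:seconds label.
; Seconds are approximated by slicing digits from the scaled fraction's string rather than using modulo, with "60" patched to "00".
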(event `/Game/Politwars/Blueprints/Logic/TimerInterface.Start_Timer`
  (bind _returnvalue (`KismetStringLibrary.Mid` (`KismetStringLibrary.Conv_DoubleToString` (/ (`self.Sec`) 1.67)) 2 2))
  (`KismetSystemLibrary.Delay` 1.0)
  (`SceneComponent.SetVisibility` (`self.TextTimer`) true false)
  (bind (_direction _timer) (`Timeline|Countdown timer` :!via `ReverseFromEnd`)
    (:`Update`
      (bind _returnvalue_2 (/ _timer 60.0))
      (set `self.Min` (`KismetMathLibrary.FFloor` _returnvalue_2))
      (set `self.Sec` (`KismetMathLibrary.Fraction` _returnvalue_2))
      (if (`KismetStringLibrary.EqualEqual_StrStr` _returnvalue "60")
        (set `self.TimerString` "00")
        (else
          (set `self.TimerString` _returnvalue)))
      (`TextRenderComponent.K2_SetText` (`self.TextTimer`) (`KismetTextLibrary.Conv_StringToText` (`KismetStringLibrary.Concat_StrStr` "Timer:" (`KismetStringLibrary.Concat_StrStr` (`KismetStringLibrary.Conv_IntToString` (`self.Min`)) (`KismetStringLibrary.Concat_StrStr` ":" (`self.TimerString`)))))))))

(event `self.ReceiveBeginPlay`)

(fn `UserConstructionScript`)