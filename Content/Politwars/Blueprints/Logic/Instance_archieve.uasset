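; Archived economy logic for a strategy game, computing a faction's fees, food, population, gold and tech from population, army and building counts.
; Plantations and academies set food and tech income, each with a bonus scaled by a god's favor (Perci, Gefest).
; Army and population drive food consumption, while army alone sets military spending.
; Food math stores its balance in FoodTransit, which a separate Transiting step copies into Food.
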(fn `Fees_Math`
  (set `self.Fees` (/ (- (`self.Population`) (`self.Army`)) 3)))

(fn `Food_Math`
  (set `self.Food_Income` (+ (* (`self.Plantations`) 500) (/ (* (* (`self.Plantations`) 500) (`KismetMathLibrary.FTrunc` (`self.Perci_Favor`))) 10000)))
  (set `self.Food_Outcome` (+ (`self.Army`) (/ (`self.Population`) 2)))
  (set `self.Food_Transit` (+ (- (`self.Food`) (`self.Food_Outcome`)) (`self.Food_Income`))))

(fn `Gold_Math`
  (set `self.Gold_Income` (/ (- (`self.Population`) (`self.Army`)) 3))
  (set `self.Military_spending` (/ (`self.Army`) 10)))

(fn `Population_Math`
  (set `self.Population` (- (- (+ (`self.Population`) (`self.Food`)) (`self.Population`)) (* 2 (`self.Army`)))))

(fn `Tech_math`
  (set `self.Tech_Income` (+ (+ (`self.Technologies`) (`KismetMathLibrary.Conv_IntToDouble` (* (`self.Academies`) 200))) (* (/ (* (`self.Academies`) 200) 10000) (`self.Gefest_Favor`)))))

(fn `Transiting`
  (set `self.Food` (`self.Food_Transit`)))