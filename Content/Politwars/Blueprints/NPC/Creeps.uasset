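; Neutral creep NPC that resolves attacks sent against it and displays its stats in a widget.
; AtackOnNPC_creeps scans each attacker's orders targeting this creep's Name, subtracting losses that scale with HP squared over troop count.
; Non-negative results add survivors, HP-scaled gold and fixed food to the attacker; otherwise a Russian defeat message prints.
; ShowUI_Creep fills the CreepValue widget with picture, HP and name.
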(fn `AtackOnNPC_creeps`
  (for _array_element (`self.NPCAtackers`)
    (for _array_element_2 (`/Game/Politwars/Blueprints/Players/Player_Polis.Atack_quantity_new` _array_element)
      (bind (_quantity _target) (break `/Game/Politwars/Blueprints/UI/Raiting_test/WarGroup` _array_element_2))
      (if (`KismetStringLibrary.EqualEqual_StrStr` _target (`self.Name`))
        (bind _returnvalue (- _quantity (`KismetMathLibrary.FTrunc` (/ (* (`KismetMathLibrary.Square` (`KismetMathLibrary.Conv_IntToDouble` (`self.HP`))) 0.8) (`KismetMathLibrary.Conv_IntToDouble` _quantity)))))
        (if (>= _returnvalue 0)
          (set `/Game/Politwars/Blueprints/Players/Player_Polis.Survivors` (+ (`/Game/Politwars/Blueprints/Players/Player_Polis.Survivors` _array_element) _returnvalue) _array_element)
          (set `/Game/Politwars/Blueprints/Players/Player_Polis.Gold` (+ (`/Game/Politwars/Blueprints/Players/Player_Polis.Gold` _array_element) (* (`self.HP`) 5)) _array_element)
          (set `/Game/Politwars/Blueprints/Players/Player_Polis.Food` (+ (`/Game/Politwars/Blueprints/Players/Player_Polis.Food` _array_element) 20) _array_element)
          (else
            (`KismetSystemLibrary.PrintString` (`KismetStringLibrary.Concat_StrStr` "Войска из " _target " погибли в стычке с нейтралами."))))))))

(fn `ShowUI_Creep`
  (bind _ascreep_value (cast `/Game/Politwars/Blueprints/UI/CreepValue` (`WidgetComponent.GetWidget` (`self.CreepUI`))))
  (`Image.SetBrushFromTexture` (`/Game/Politwars/Blueprints/UI/CreepValue.CreaturePic` _ascreep_value) (`self.CreepPic`) false)
  (`TextBlock.SetText` (`/Game/Politwars/Blueprints/UI/CreepValue.BossHPText` _ascreep_value) (`KismetTextLibrary.Conv_IntToText` (`self.HP`) false false))
  (`TextBlock.SetText` (`/Game/Politwars/Blueprints/UI/CreepValue.Minotaur` _ascreep_value) (`KismetTextLibrary.Conv_StringToText` (`self.Name`))))

(fn `UserConstructionScript`
  (`parent.UserConstructionScript`))