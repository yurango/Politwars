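; Boss NPC that resolves combined squad attacks and shows its name, HP and bounty in a BossValue widget filled at BeginPlay.
; AtackOnNPCBoss sums attacks targeting it by name, subtracting them from HP if the boss survives.
; On defeat it updates attackers' survivors, gold and food, resets the bounty and scales HP by resurrection count, all inside the per-attack reward loop.
; The attacker list is cleared after each resolution.
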(event `self.ReceiveBeginPlay`
  (`self.ShowUI`))

(fn `AtackOnNPC_boss`
  (locals (SquadAtack :type Integer) (SquadQuantity :type Integer))
  (bind _npcatackers (`self.NPCAtackers`))
  (bind _resurrectionquantity (`self.ResurrectionQuantity`))
  (for _array_element _npcatackers
    (for _array_element_2 (`/Game/Politwars/Blueprints/Players/Player_Polis.Atack_quantity_new` _array_element)
      (bind (_quantity _target) (break `/Game/Politwars/Blueprints/UI/Raiting_test/WarGroup` _array_element_2))
      (if (`KismetStringLibrary.EqualEqual_StrStr` _target (`self.Name`))
        (set `local.SquadAtack` (+ (`local.SquadAtack`) _quantity))
        (`/Engine/EditorBlueprintResources/StandardMacros.IncrementInt` (`local.SquadQuantity`)))))
  (if (>= (`local.SquadAtack`) (`self.HP`))
    (`KismetSystemLibrary.PrintString` "Босс повержен" false true (struct :`G` 0.66 :`B` 1.0 :`A` 1.0) 5.0)
    (for _array_element_3 (`self.NPCAtackers`)
      (for _array_element_4 (`/Game/Politwars/Blueprints/Players/Player_Polis.Atack_quantity_new` _array_element_3)
        (bind (_quantity_2 _target_2) (break `/Game/Politwars/Blueprints/UI/Raiting_test/WarGroup` _array_element_4))
        (if (`KismetStringLibrary.EqualEqual_StrStr` _target_2 (`self.Name`))
          (set `/Game/Politwars/Blueprints/Players/Player_Polis.Survivors` (+ (`/Game/Politwars/Blueprints/Players/Player_Polis.Survivors` _array_element_3) (* (`KismetMathLibrary.FTrunc` (/ (`KismetMathLibrary.Conv_IntToDouble` (- (`local.SquadAtack`) (`self.HP`))) (`KismetMathLibrary.Conv_IntToDouble` (`local.SquadAtack`)))) _quantity_2)) _array_element_3)
          (set `/Game/Politwars/Blueprints/Players/Player_Polis.Gold` (+ (`/Game/Politwars/Blueprints/Players/Player_Polis.Gold` _array_element_3) (/ (`self.Bounty`) (`local.SquadQuantity`))) _array_element_3)
          (set `/Game/Politwars/Blueprints/Players/Player_Polis.Food` (+ (`/Game/Politwars/Blueprints/Players/Player_Polis.Food` _array_element_3) (/ (`self.HP`) (`local.SquadQuantity`))) _array_element_3)
          (set `self.Bounty` (`self.DefaultBounty`))
          (`/Engine/EditorBlueprintResources/StandardMacros.IncrementInt` _resurrectionquantity
            (:`  `
              (set `self.HP` (* _resurrectionquantity (`KismetMathLibrary.FTrunc` (* (`self.DefaultHP`) 1.5))))
              (set `local.SquadAtack` 0)
              (set `local.SquadQuantity` 0))))))
    (else
      (`KismetSystemLibrary.PrintString` "Босс выстоял" false true (struct :`G` 0.66 :`B` 1.0 :`A` 1.0) 5.0)
      (set `self.HP` (- (`self.HP`) (`local.SquadAtack`)))))
  (`KismetArrayLibrary.Array_Clear` _npcatackers)
  (set `local.SquadAtack` 0)
  (set `local.SquadQuantity` 0))

(fn `ShowUI`
  (bind _asboss_value (cast `/Game/Politwars/Blueprints/UI/BossValue` (`WidgetComponent.GetWidget` (`self.BossStatusUI`))))
  (`TextBlock.SetText` (`/Game/Politwars/Blueprints/UI/BossValue.BossBountyText` _asboss_value) (`KismetTextLibrary.Conv_IntToText` (`self.Bounty`) false false))
  (`TextBlock.SetText` (`/Game/Politwars/Blueprints/UI/BossValue.BossHPText` _asboss_value) (`KismetTextLibrary.Conv_IntToText` (`self.HP`) false false))
  (`TextBlock.SetText` (`/Game/Politwars/Blueprints/UI/BossValue.Minotaur` _asboss_value) (`KismetTextLibrary.Conv_StringToText` (`self.Name`))))

(fn `UserConstructionScript`
  (`parent.UserConstructionScript`))