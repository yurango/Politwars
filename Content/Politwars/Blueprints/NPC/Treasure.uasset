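; Treasure NPC that resolves attacks on it and pays out its HP as gold.
; AtackOnTreasure first totals attack quantities aimed at its Name into Danger and tracks the largest.
; BiggestName stores that attack's target, not the attacker, so the second pass matches attacks by target.
; Matches gain the gold, print a Russian capture message and keep all troops; other entries add survivors scaled against Danger.
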(fn `AtackOnTreasure`
  (locals (Biggest :type Integer) (Danger :type Integer) (BiggestName :type String))
  (for _array_element (`self.NPCAtackers`)
    (for _array_element_2 (`/Game/Politwars/Blueprints/Players/Player_Polis.Atack_quantity_new` _array_element)
      (bind (_quantity _target) (break `/Game/Politwars/Blueprints/UI/Raiting_test/WarGroup` _array_element_2))
      (if (`KismetStringLibrary.EqualEqual_StrStr` _target (`self.Name`))
        (set `local.Danger` (+ (`local.Danger`) _quantity))
        (if (> _quantity (`local.Biggest`))
          (set `local.Biggest` _quantity)
          (set `local.BiggestName` _target)))))
  (for _array_element_3 (`self.NPCAtackers`)
    (for _array_element_4 (`/Game/Politwars/Blueprints/Players/Player_Polis.Atack_quantity_new` _array_element_3)
      (bind (_quantity_2 _target_2) (break `/Game/Politwars/Blueprints/UI/Raiting_test/WarGroup` _array_element_4))
      (if (`KismetStringLibrary.EqualEqual_StrStr` _target_2 (`local.BiggestName`))
        (set `/Game/Politwars/Blueprints/Players/Player_Polis.Gold` (+ (`/Game/Politwars/Blueprints/Players/Player_Polis.Gold` _array_element_3) (`self.HP`)) _array_element_3)
        (`KismetSystemLibrary.PrintString` (`KismetStringLibrary.Concat_StrStr` "Войска из " _target " присвоили себе сокровища."))
        (set `/Game/Politwars/Blueprints/Players/Player_Polis.Survivors` (+ (`/Game/Politwars/Blueprints/Players/Player_Polis.Survivors` _array_element_3) _quantity_2) _array_element_3)
        (else
          (set `/Game/Politwars/Blueprints/Players/Player_Polis.Survivors` (+ (`/Game/Politwars/Blueprints/Players/Player_Polis.Survivors` _array_element_3) (`KismetMathLibrary.FTrunc` (* _quantity_2 (/ (`KismetMathLibrary.Conv_IntToDouble` _quantity_2) (* (`KismetMathLibrary.Conv_IntToDouble` (`local.Danger`)) 0.75))))) _array_element_3))))))

(fn `UserConstructionScript`
  (`parent.UserConstructionScript`))