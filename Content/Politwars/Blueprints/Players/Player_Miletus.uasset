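; Player Blueprint for Miletus that lets input actions grow or shrink a clipart sprite serving as the city icon.
; The Bigger City and Smaller City actions step IconSize up or down by a fixed amount, unclamped, and apply it as the sprite's uniform world scale.
; Only the Bigger City action sets the sprite component to replicate, and neither uses an RPC.
; The construction script just calls its parent.
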(event `InputAction|Bigger City`
  (params (Key :type "Key Structure"))
  (:`Pressed`
    (`ActorComponent.SetIsReplicated` (`self.PinClipart_com_clipper-cutty-sark_3965685_Sprite`) true)
    (bind _output_get (set `self.Icon Size` (+ (`self.Icon Size`) 0.025)))
    (`SceneComponent.SetWorldScale3D` (`self.PinClipart_com_clipper-cutty-sark_3965685_Sprite`) (+ (0.0 0.0 0.0) _output_get))))

(event `InputAction|Smaller City`
  (params (Key :type "Key Structure"))
  (:`Pressed`
    (bind _output_get (set `self.Icon Size` (+ (`self.Icon Size`) -0.025)))
    (`SceneComponent.SetWorldScale3D` (`self.PinClipart_com_clipper-cutty-sark_3965685_Sprite`) (+ (0.0 0.0 0.0) _output_get))))

(fn `UserConstructionScript`
  (`parent.UserConstructionScript`))