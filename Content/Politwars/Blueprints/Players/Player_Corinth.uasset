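; Player blueprint for Corinth that lets input resize the city's sprite.
; The Bigger City and Smaller City actions step IconSize up or down by a fixed amount, then apply it as a uniform world scale on CorinthSprite.
; IconSize has no clamping here, and the construction script only calls its parent.
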(event `InputAction|Bigger City`
  (params (Key :type "Key Structure"))
  (:`Pressed`
    (bind _output_get (set `self.Icon Size` (+ (`self.Icon Size`) 0.1)))
    (`SceneComponent.SetWorldScale3D` (`self.corinth_Sprite`) (+ (0.0 0.0 0.0) _output_get))))

(event `InputAction|Smaller City`
  (params (Key :type "Key Structure"))
  (:`Pressed`
    (bind _output_get (set `self.Icon Size` (+ (`self.Icon Size`) -0.1)))
    (`SceneComponent.SetWorldScale3D` (`self.corinth_Sprite`) (+ (0.0 0.0 0.0) _output_get))))

(fn `UserConstructionScript`
  (`parent.UserConstructionScript`))